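; KeyPort is a spinning key pickup that enables a linked lockable port.
; When an actor of the Movement class overlaps it, it sets CheckKeyPickup on the LockablePort referenced by KeyForThisDoor, destroys itself and plays a key sound.
; Each tick it rotates its scene component around the vertical axis, at a rate tied to frame rate rather than delta time.
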(event EventTick
  (params (DeltaSeconds :type Float%20%28single-precision%29))
  (Transformation|AddWorldRotation (Variables|Default|GetScene) "0,1.500000,0.000000" false false))

(event Collision|EventActorBeginOverlap
  (params (OtherActor :type Actor%20Object%20Reference))
  (if (== "/Game/Blueprint/Movement.Movement_C" (Utilities|GetClass OtherActor))
    (bind _aslockable_port (Utilities|Casting|CastToLockablePort (Variables|Default|GetKeyForThisDoor)))
    (Variables|/Game/Blueprint/LockablePort.LockablePort_C|SetCheck%20key%20pickup _aslockable_port true)
    (Actor|DestroyActor)
    (Audio|PlaySound2D "/Game/Sound/Foley/Keys.Keys" 1.0 1.0 0.0 0 0)))

(fn ConstructionScript)