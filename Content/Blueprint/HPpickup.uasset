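; Health pickup actor that grants the player health on overlap and spins in the world.
; When the overlapping actor's class is Movement, it casts its Player reference, not the overlapping actor, to Movement.
; If PlayerHealth is at most 99, it adds 10 without clamping, destroys itself and plays a 2D sound.
; Tick yaws the Scene component by a fixed step each frame, unscaled by delta time.
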(event Collision|EventActorBeginOverlap
  (params (OtherActor :type Actor%20Object%20Reference))
  ;[1 1 1] Allows the player to get health and then gets deleted
  (if (== "/Game/Blueprint/Movement.Movement_C" (Utilities|GetClass OtherActor))
    (bind _asmovement (Utilities|Casting|CastToMovement (Variables|Default|GetPlayer)))
    (if (<= (Variables|/Game/Blueprint/Movement.Movement_C|GetPlayerHealth _asmovement) 99)
      (Variables|/Game/Blueprint/Movement.Movement_C|SetPlayerHealth _asmovement (+ (Variables|/Game/Blueprint/Movement.Movement_C|GetPlayerHealth _asmovement) 10))
      (Actor|DestroyActor)
      (Audio|PlaySound2D "/Game/Sound/Foley/HealthPickup1.HealthPickup1" 1.0 1.0 0.0 0 0))))

(event EventTick
  (params (DeltaSeconds :type Float%20%28single-precision%29))
  (Transformation|AddWorldRotation (Variables|Default|GetScene) "0,1.500000, 0" false false))

(fn ConstructionScript)