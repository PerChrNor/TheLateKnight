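; Trigger actor for the Patrick encounter, handling his dialog and the handover of armour.
; On overlap it casts the player character to Movement, plays Dialog10 on the DialogController and calls MoreDamage on every BpEnemyCPP.
; RemoveArmor, with no caller in this graph, calls Patrick on that Movement, changes PatrickModel's stance and unhides the Armor and Sword.
; It then destroys PatrickDialog and itself.
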(event Custom|Remove%20Armor
  ;[1 1 1] giving patrick armour and dialog
  (Default|Patrick (stale Collision|EventActorBeginOverlap _asmovement))
  (bind _aspatrick_model (Utilities|Casting|CastToPatrickModel (Variables|Default|GetPatrickModel)))
  (Default|ChangeStance _aspatrick_model)
  (Rendering|SetActorHiddenInGame (Variables|Default|GetArmor) false)
  (Actor|DestroyActor (Variables|Default|GetPatrickDialog))
  (Actor|DestroyActor))

(event Collision|EventActorBeginOverlap
  (params (OtherActor :type Actor%20Object%20Reference))
  ;[1 1 1] giving patrick armour and dialog
  (bind _asmovement (Utilities|Casting|CastToMovement (Game|GetPlayerCharacter 0)))
  (bind _asdialog_controller (Utilities|Casting|CastToDialogController (Variables|Default|GetDialogController)))
  (Default|Dialog10 _asdialog_controller)
  (bind _outactors (Actor|GetAllActorsOfClass "/Game/Blueprint/bpEnemyCPP.bpEnemyCPP_C"))
  (for _array_element _outactors
    (Default|MoreDamage _array_element)))

(fn ConstructionScript)