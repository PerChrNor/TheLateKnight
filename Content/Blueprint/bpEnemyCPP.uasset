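; Goat enemy that damages the player on contact and can be hurt and killed by the player.
; Overlaps with the player's capsule in its Box apply cooldown-gated damage, which MoreDamage can change.
; Player hits reduce health, update the percentage for the owner-linked health bar widget and knock the goat back with a swept offset.
; Attack, hit and death events set timed ABPGoat flags, with death disabling collision before destroying the actor.
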(event Custom|Death%20Anim
  ;[1 1 1] Setting up animations for the goat
  (bind _asabpgoat (Utilities|Casting|CastToABPGoat (Components|SkeletalMesh|GetAnimInstance (Variables|Default|GetSkeletalMesh))))
  (Variables|/Game/Blueprint/AnimationBlueprint/ABPGoat.ABPGoat_C|SetDeath _asabpgoat true)
  (Utilities|FlowControl|Delay 0.8)
  (Actor|DestroyActor))

(event Custom|Attack%20Anim
  ;[1 1 1] Setting up animations for the goat
  (bind _asabpgoat (Utilities|Casting|CastToABPGoat (Components|SkeletalMesh|GetAnimInstance (Variables|Default|GetSkeletalMesh))))
  (Variables|/Game/Blueprint/AnimationBlueprint/ABPGoat.ABPGoat_C|SetIsAttacking _asabpgoat true)
  (Utilities|FlowControl|Delay 0.5)
  (Variables|/Game/Blueprint/AnimationBlueprint/ABPGoat.ABPGoat_C|SetIsAttacking _asabpgoat false))

(event Custom|Damaged%20Anim
  ;[1 1 1] Setting up animations for the goat
  (bind _asabpgoat (Utilities|Casting|CastToABPGoat (Components|SkeletalMesh|GetAnimInstance (Variables|Default|GetSkeletalMesh))))
  (Variables|/Game/Blueprint/AnimationBlueprint/ABPGoat.ABPGoat_C|SetGotHit _asabpgoat true)
  (Utilities|FlowControl|Delay 0.25)
  (Variables|/Game/Blueprint/AnimationBlueprint/ABPGoat.ABPGoat_C|SetGotHit _asabpgoat false))

(event Custom|More%20Damage
  (Variables|Default|SetEnemy%20Damage 3e+01))

(event Game|Damage|EventAnyDamage
  (params (Damage :type Float%20%28single-precision%29) (DamageType :type Damage%20Type%20Object%20Reference) (InstigatedBy :type Controller%20Object%20Reference) (DamageCauser :type Actor%20Object%20Reference))
  (bind _returnvalue (Transformation|GetActorRotation))
  (bind _returnvalue_2 (Math|Vector|GetForwardVector _returnvalue))
  (bind _returnvalue_3 (* _returnvalue_2 -3e+02))
  (bind (_x _y) (Math|Vector|BreakVector _returnvalue_3))
  ;[1 1 1] Enemy taking damage and HUD
  (bind _output_get (Variables|Default|SetDamaged%20By%20player (== (Utilities|GetClass DamageCauser) (Utilities|GetClass (Game|GetPlayerCharacter 0)))))
  (if _output_get
    (Variables|Default|SetEnemy%20Health (- (Variables|Default|GetEnemy%20Health) (Math|Float|Truncate Damage)))
    (CallFunction|SetHPBar)
    (CallFunction|DamagedAnim)
    (Transformation|AddWorldOffset (Variables|Default|GetCollisionSphereEnemy) (Math|Vector|MakeVector _x _y 0.0) true false)
    (Math|Integer|CompareInt (Variables|Default|GetEnemy%20Health)
      (:==
        _)
      (:<
        _))
    (CallFunction|DeathAnim)
    (Collision|SetCollisionEnabled (Variables|Default|GetCollisionSphereEnemy) "NoCollision")))

(event Collision|EventActorBeginOverlap
  (params (OtherActor :type Actor%20Object%20Reference))
  ;[1 1 1] enemy damage delay
  (bind _output_get (Variables|Default|Setis%20player (Utilities|Array|ContainsItem (Class|PrimitiveComponent|GetOverlappingComponents (Variables|Default|GetBox)) (Variables|Default|GetSavedCapsule))))
  (if _output_get
    (if (Variables|Default|Getready%20to%20dmg)
      (Variables|Default|Setready%20to%20dmg false)
      (Game|Damage|ApplyDamage OtherActor (Variables|Default|GetEnemy%20Damage) 0 self)
      (CallFunction|AttackAnim)
      (Utilities|FlowControl|Delay 0.2)
      (Variables|Default|Setready%20to%20dmg true))))

(event EventBeginPlay
  ;[1 1 1] hud health setup
  (bind _asenemyhealth (Utilities|Casting|CastToEnemyhealth (UserInterface|GetUserWidgetObject (Variables|Default|Gethealthbar))))
  (Variables|/Game/Blueprint/Enemyhealth.Enemyhealth_C|SetOwner _asenemyhealth self)
  (Variables|Default|SetSavedCapsule (Actor|GetComponentbyClass (Game|GetPlayerCharacter 0) "/Script/Engine.CapsuleComponent")))

(fn ConstructionScript)

(fn SetHPBar
  (Variables|Default|SetHP%20Percent (Math|Float|Clamp(Float) (/ (Math|Conversions|ToFloat(Integer) (Variables|Default|GetEnemy%20Health)) 1e+02))))