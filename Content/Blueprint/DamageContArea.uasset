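; Continuous damage area actor that repeatedly hurts the player while they overlap it.
; Begin and end overlap compare the other actor's class to the player character's, toggling a CurrentlyDmging flag.
; Begin overlap starts a delay-based loop that applies fixed damage to player 0 until the flag clears.
; A CheckDmgable health check exists but is never called here, and its while condition is false.
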(event Custom|ContinusDMG
  ;[1 1 1] Applying damage when player overlap
  (Game|Damage|ApplyDamage (Game|GetPlayerCharacter 0) 5.0 0 0 :!label _label)
  (Utilities|FlowControl|Delay 0.1)
  (if (Variables|Default|GetCurrentlyDmging)
    (goto _label)))

(event Collision|EventActorBeginOverlap
  (params (OtherActor :type Actor%20Object%20Reference))
  ;[1 1 1] Applying damage when player overlap
  (bind _output_get (Variables|Default|Setdamaging%20player (== (Utilities|GetClass OtherActor) (Utilities|GetClass (Game|GetPlayerCharacter 0)))))
  (if _output_get
    (Variables|Default|SetCurrentlyDmging true)
    (CallFunction|ContinusDMG)))

(event Collision|EventActorEndOverlap
  (params (OtherActor :type Actor%20Object%20Reference))
  ;[1 1 1] Applying damage when player overlap
  (bind _output_get (Variables|Default|Setdamaging%20player (== (Utilities|GetClass OtherActor) (Utilities|GetClass (Game|GetPlayerCharacter 0)))))
  (if _output_get
    (Variables|Default|SetCurrentlyDmging false)))

(fn ConstructionScript)

(fn CheckDmgable
  (while false :!label _label
    (bind _asmovement (Utilities|Casting|CastToMovement (Game|GetPlayerCharacter 0)))
    (Math|Integer|CompareInt (Variables|/Game/Blueprint/Movement.Movement_C|GetPlayerHealth _asmovement)
      (:>
        (Variables|Default|SetCurrentlyDmging true)
        (goto _label))
      (:==
        _)
      (:<
        _))
    (Variables|Default|SetCurrentlyDmging false)
    (goto _label)))