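; WallControll is a trigger actor that switches the visibility of sets of actors, noted as walls that block the player's view.
; On actor begin overlap, it checks whether the player character's capsule is among the components overlapping its Box.
; If so, it hides every actor in Hiddenarray and shows every actor in NotHiddenArray.
; There is no end-overlap handling, so leaving the box does not revert the change.
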(event Collision|EventActorBeginOverlap
  (params (OtherActor :type Actor%20Object%20Reference))
  ;[1 1 1] walls so u cannot see
  (bind _output_get (Variables|Default|Setis%20player (Utilities|Array|ContainsItem (Class|PrimitiveComponent|GetOverlappingComponents (Variables|Default|GetBox)) (Actor|GetComponentbyClass (Game|GetPlayerCharacter 0) "/Script/Engine.CapsuleComponent"))))
  (if _output_get
    (for _array_element (Variables|Default|GetHiddenarray)
      (Rendering|SetActorHiddenInGame _array_element true))
    (for _array_element_2 (Variables|Default|GetNot%20Hidden%20Array)
      (Rendering|SetActorHiddenInGame _array_element_2 false))))

(fn ConstructionScript)