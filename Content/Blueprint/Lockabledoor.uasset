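; Lockable door actor that swings open on player interaction, provided its CheckKeyPickup flag is set.
; Overlap toggles a widget, shown only while the door is closed and hidden on leaving or opening.
; Opening disables the Cube's collision and uses a timeline to rotate the actor -90 degrees in yaw from its starting rotation.
; A PlaySound flag limits the opening sound to one play, located at the world origin.
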(event Custom|Opendoor
  ;[1 1 1] Rotates and disable the collision so the player can walk through the door
  (if (Variables|Default|GetCheck%20key%20pickup)
    (Variables|Default|Setdoor%20is%20open true)
    (Collision|SetCollisionEnabled (Variables|Default|GetCube) "NoCollision")
    (bind _dooropener (Timeline|Timeline_0 Play)
      (:Update
        (Transformation|SetActorRotation (Math|Rotator|Lerp(Rotator) (Variables|Default|GetObject%20Rotation) (Variables|Default|GetRotator%20of%20this%20obj) _dooropener))
        (if (Variables|Default|GetPlay%20Sound)
          (Audio|PlaySoundatLocation "/Game/Sound/Foley/DoorOpening_Cue.DoorOpening_Cue" "0, 0, 0" "0, 0, 0" 1.0 1.0 0.0 0 0 0)
          (Variables|Default|SetPlay%20Sound false))))))

(event Collision|EventActorEndOverlap
  (params (OtherActor :type Actor%20Object%20Reference))
  (Rendering|SetVisibility (Variables|Default|GetWidget) false false))

(event EventOnPlayerInteract
  ;[1 1 1] Player interaction
  (CallFunction|Opendoor)
  (if (Variables|Default|Getdoor%20is%20open)
    (Rendering|SetVisibility (Variables|Default|GetWidget) false false)))

(event Collision|EventActorBeginOverlap
  (params (OtherActor :type Actor%20Object%20Reference))
  ;[1 1 1] widget visibility
  (if (Variables|Default|Getdoor%20is%20open)
    (Rendering|SetVisibility (Variables|Default|GetWidget) false false)
    (else
      (Rendering|SetVisibility (Variables|Default|GetWidget) true false))))

(event EventBeginPlay
  (bind _returnvalue (Transformation|GetActorRotation))
  (bind (_roll _pitch _yaw) (Math|Rotator|BreakRotator _returnvalue))
  (Variables|Default|SetObject%20Rotation _returnvalue)
  (Variables|Default|SetRotator%20of%20this%20obj (Math|Rotator|MakeRotator _roll _pitch (+ _yaw -9e+01))))

(fn ConstructionScript)