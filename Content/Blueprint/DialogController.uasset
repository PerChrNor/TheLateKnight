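; DialogController holds the game's hardcoded conversations and inspect texts: Potato Boi's controls hint, a painting, gravestones and Patrick's armor request.
; Each DialogN event call advances a shared Talkint counter and writes the next line to the player Movement character's Dialog variable.
; Every call runs StartDialog, adding another DialogBoxHUD and disabling movement; EndDialog removes all boxes and restores movement.
; Finishing Patrick's conversation also calls RemoveArmor on him.
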(event Custom|StartDialog
  (bind _returnvalue (UserInterface|CreateWidget "/Game/Blueprint/DialogBoxHUD.DialogBoxHUD_C" (Game|GetPlayerController 0)))
  (UserInterface|Viewport|AddtoViewport _returnvalue 0)
  (bind _asmovement (Utilities|Casting|CastToMovement (Game|GetPlayerCharacter 0)))
  (Default|DisableMovement _asmovement))

(event Custom|Dialog10
  (bind _returnvalue (Game|GetPlayerCharacter 0))
  (CallFunction|StartDialog)
  (if (== (Variables|Default|Gettalkint) 0)
    (bind _asmovement (Utilities|Casting|CastToMovement _returnvalue))
    (Variables|/Game/Blueprint/Movement.Movement_C|SetDialog _asmovement "Patrick: 
“Greetings good sir. It is I, Sir Patrick the Same. 
I would like to use your garb in my quest for my fair princess. May I undress you?”")
    (Variables|Default|Settalkint 1)
    (elif (== (Variables|Default|Gettalkint) 1)
      (bind _asmovement_2 (Utilities|Casting|CastToMovement _returnvalue))
      (Variables|/Game/Blueprint/Movement.Movement_C|SetDialog _asmovement_2 "Chaster: 
“Pardon?” ")
      (Variables|Default|Settalkint 2)
      (elif (== (Variables|Default|Gettalkint) 2)
        (bind _asmovement_3 (Utilities|Casting|CastToMovement _returnvalue))
        (Variables|/Game/Blueprint/Movement.Movement_C|SetDialog _asmovement_3 "Patrick:  
“Well, you struck outeth with thy princesseth, you don’t need itth anymoreth.”")
        (Variables|Default|Settalkint 3)
        (elif (== (Variables|Default|Gettalkint) 3)
          (bind _asmovement_4 (Utilities|Casting|CastToMovement _returnvalue))
          (Variables|/Game/Blueprint/Movement.Movement_C|SetDialog _asmovement_4 "Chaster: 
I don’t think you understand how English works.”")
          (Variables|Default|Settalkint 4)
          (elif (== (Variables|Default|Gettalkint) 4)
            (bind _asmovement_5 (Utilities|Casting|CastToMovement _returnvalue))
            (Variables|/Game/Blueprint/Movement.Movement_C|SetDialog _asmovement_5 "Patrick: 
“Quicketh! The nighteth is runneth lateth. I needeth that armour and sword… eth.” ")
            (Variables|Default|Settalkint 5)
            (elif (== (Variables|Default|Gettalkint) 5)
              (bind _asmovement_6 (Utilities|Casting|CastToMovement _returnvalue))
              (Variables|/Game/Blueprint/Movement.Movement_C|SetDialog _asmovement_6 "Chaster: 
“Alright, fine! Just stop torturing the English language! Shakespeare (who is alive currently)  
does not deserve this.” ")
              (Variables|Default|Settalkint 6)
              (elif (== (Variables|Default|Gettalkint) 6)
                (bind _asmovement_7 (Utilities|Casting|CastToMovement _returnvalue))
                (Variables|/Game/Blueprint/Movement.Movement_C|SetDialog _asmovement_7 "Patrick:  
“Thanketh thee, Here is a stick-eth, Sir Whats-your-face! Good Day!” ")
                (Variables|Default|Settalkint 7)
                (elif (== (Variables|Default|Gettalkint) 7)
                  (Variables|Default|Settalkint 0)
                  (CallFunction|EndDialog)
                  (bind _aspatrick (Utilities|Casting|CastToPatrick (Variables|Default|GetPatrick)))
                  (Default|RemoveArmor _aspatrick))))))))))

(event Custom|Dialog4
  (bind _returnvalue (Game|GetPlayerCharacter 0))
  ;[1 1 1] Gravestones
  (CallFunction|StartDialog)
  (if (== (Variables|Default|Gettalkint) 0)
    (bind _asmovement (Utilities|Casting|CastToMovement _returnvalue))
    (Variables|/Game/Blueprint/Movement.Movement_C|SetDialog _asmovement "Here lies Eira ")
    (Variables|Default|Settalkint 1)
    (elif (== (Variables|Default|Gettalkint) 1)
      (bind _asmovement_2 (Utilities|Casting|CastToMovement _returnvalue))
      (Variables|/Game/Blueprint/Movement.Movement_C|SetDialog _asmovement_2 "The first 4 words were too much.")
      (Variables|Default|Settalkint 2)
      (elif (== (Variables|Default|Gettalkint) 2)
        (Variables|Default|Settalkint 0)
        (CallFunction|EndDialog)))))

(event Custom|Dialog5
  (bind _returnvalue (Game|GetPlayerCharacter 0))
  ;[1 1 1] Gravestones
  (CallFunction|StartDialog)
  (if (== (Variables|Default|Gettalkint) 0)
    (bind _asmovement (Utilities|Casting|CastToMovement _returnvalue))
    (Variables|/Game/Blueprint/Movement.Movement_C|SetDialog _asmovement "Here lies Nathalie")
    (Variables|Default|Settalkint 1)
    (elif (== (Variables|Default|Gettalkint) 1)
      (bind _asmovement_2 (Utilities|Casting|CastToMovement _returnvalue))
      (Variables|/Game/Blueprint/Movement.Movement_C|SetDialog _asmovement_2 "She was banished to the Ghost Dimension after shitposting too much.")
      (Variables|Default|Settalkint 2)
      (elif (== (Variables|Default|Gettalkint) 2)
        (Variables|Default|Settalkint 0)
        (CallFunction|EndDialog)))))

(event Custom|Dialog6
  (bind _returnvalue (Game|GetPlayerCharacter 0))
  ;[1 1 1] Gravestones
  (CallFunction|StartDialog)
  (if (== (Variables|Default|Gettalkint) 0)
    (bind _asmovement (Utilities|Casting|CastToMovement _returnvalue))
    (Variables|/Game/Blueprint/Movement.Movement_C|SetDialog _asmovement "Here lies Miriam ")
    (Variables|Default|Settalkint 1)
    (elif (== (Variables|Default|Gettalkint) 1)
      (bind _asmovement_2 (Utilities|Casting|CastToMovement _returnvalue))
      (Variables|/Game/Blueprint/Movement.Movement_C|SetDialog _asmovement_2 "She didn't know that exposure couldn't pay the bills and was executed for tax evasion. ")
      (Variables|Default|Settalkint 2)
      (elif (== (Variables|Default|Gettalkint) 2)
        (Variables|Default|Settalkint 0)
        (CallFunction|EndDialog)))))

(event Custom|Dialog1
  (bind _returnvalue (Game|GetPlayerCharacter 0))
  (CallFunction|StartDialog)
  (if (== (Variables|Default|Gettalkint) 0)
    (bind _asmovement (Utilities|Casting|CastToMovement _returnvalue))
    (Variables|/Game/Blueprint/Movement.Movement_C|SetDialog _asmovement "Potato Boi: Need help, huh? ")
    (Variables|Default|Settalkint 1)
    (elif (== (Variables|Default|Gettalkint) 1)
      (bind _asmovement_2 (Utilities|Casting|CastToMovement _returnvalue))
      (Variables|/Game/Blueprint/Movement.Movement_C|SetDialog _asmovement_2 "Potato Boi:  
It's spacebar to jump and right click to dash.  
Have fun playing the game! ")
      (Variables|Default|Settalkint 2)
      (elif (== (Variables|Default|Gettalkint) 2)
        (bind _asmovement_3 (Utilities|Casting|CastToMovement _returnvalue))
        (Variables|/Game/Blueprint/Movement.Movement_C|SetDialog _asmovement_3 "Chaster: Thanks! Wait, game?")
        (Variables|Default|Settalkint 3)
        (elif (== (Variables|Default|Gettalkint) 3)
          (bind _asmovement_4 (Utilities|Casting|CastToMovement _returnvalue))
          (Variables|/Game/Blueprint/Movement.Movement_C|SetDialog _asmovement_4 "Potato Boi: Bye!")
          (Variables|Default|Settalkint 4)
          (elif (== (Variables|Default|Gettalkint) 4)
            (Variables|Default|Settalkint 0)
            (CallFunction|EndDialog)))))))

(event Custom|Dialog7
  (bind _returnvalue (Game|GetPlayerCharacter 0))
  ;[1 1 1] Gravestones
  (CallFunction|StartDialog)
  (if (== (Variables|Default|Gettalkint) 0)
    (bind _asmovement (Utilities|Casting|CastToMovement _returnvalue))
    (Variables|/Game/Blueprint/Movement.Movement_C|SetDialog _asmovement "Here lies the remains of Per Christian")
    (Variables|Default|Settalkint 1)
    (elif (== (Variables|Default|Gettalkint) 1)
      (bind _asmovement_2 (Utilities|Casting|CastToMovement _returnvalue))
      (Variables|/Game/Blueprint/Movement.Movement_C|SetDialog _asmovement_2 "He was eaten by bugs. ")
      (Variables|Default|Settalkint 2)
      (elif (== (Variables|Default|Gettalkint) 2)
        (Variables|Default|Settalkint 0)
        (CallFunction|EndDialog)))))

(event Custom|Dialog8
  (bind _returnvalue (Game|GetPlayerCharacter 0))
  ;[1 1 1] Gravestones
  (CallFunction|StartDialog)
  (if (== (Variables|Default|Gettalkint) 0)
    (bind _asmovement (Utilities|Casting|CastToMovement _returnvalue))
    (Variables|/Game/Blueprint/Movement.Movement_C|SetDialog _asmovement "Here lies Dr. Hillestad ")
    (Variables|Default|Settalkint 1)
    (elif (== (Variables|Default|Gettalkint) 1)
      (bind _asmovement_2 (Utilities|Casting|CastToMovement _returnvalue))
      (Variables|/Game/Blueprint/Movement.Movement_C|SetDialog _asmovement_2 "He showed that chickens and dragons can indeed be one. Unfortunately. ")
      (Variables|Default|Settalkint 2)
      (elif (== (Variables|Default|Gettalkint) 2)
        (Variables|Default|Settalkint 0)
        (CallFunction|EndDialog)))))

(event Custom|Dialog9
  (bind _returnvalue (Game|GetPlayerCharacter 0))
  ;[1 1 1] Gravestones
  (CallFunction|StartDialog)
  (if (== (Variables|Default|Gettalkint) 0)
    (bind _asmovement (Utilities|Casting|CastToMovement _returnvalue))
    (Variables|/Game/Blueprint/Movement.Movement_C|SetDialog _asmovement "Here lies Fredrik")
    (Variables|Default|Settalkint 1)
    (elif (== (Variables|Default|Gettalkint) 1)
      (bind _asmovement_2 (Utilities|Casting|CastToMovement _returnvalue))
      (Variables|/Game/Blueprint/Movement.Movement_C|SetDialog _asmovement_2 "How could this happen to me, I made my mistakes, got nowhere to run, knight goes on as im fading away.")
      (Variables|Default|Settalkint 2)
      (elif (== (Variables|Default|Gettalkint) 2)
        (Variables|Default|Settalkint 0)
        (CallFunction|EndDialog)))))

(event Custom|End%20Dialog
  (bind _asmovement (Utilities|Casting|CastToMovement (Game|GetPlayerCharacter 0)))
  (Default|EnableMovement _asmovement)
  (bind _foundwidgets (Widget|GetAllWidgetsOfClass "/Game/Blueprint/DialogBoxHUD.DialogBoxHUD_C" true))
  (for _array_element _foundwidgets
    (Widget|RemovefromParent _array_element)))

(event Custom|Dialog2
  (bind _returnvalue (Game|GetPlayerCharacter 0))
  (CallFunction|StartDialog)
  (if (== (Variables|Default|Gettalkint) 0)
    (bind _asmovement (Utilities|Casting|CastToMovement _returnvalue))
    (Variables|/Game/Blueprint/Movement.Movement_C|SetDialog _asmovement "It's a painting of Princess Genevieve Maawd. She's so beautiful and majestic. ")
    (Variables|Default|Settalkint 1)
    (elif (== (Variables|Default|Gettalkint) 1)
      (bind _asmovement_2 (Utilities|Casting|CastToMovement _returnvalue))
      (Variables|/Game/Blueprint/Movement.Movement_C|SetDialog _asmovement_2 "Better run away before Chaster starts crying.")
      (Variables|Default|Settalkint 2)
      (elif (== (Variables|Default|Gettalkint) 2)
        (Variables|Default|Settalkint 0)
        (CallFunction|EndDialog)))))

(event Custom|Dialog3
  (bind _returnvalue (Game|GetPlayerCharacter 0))
  ;[1 1 1] Gravestones
  (CallFunction|StartDialog)
  (if (== (Variables|Default|Gettalkint) 0)
    (bind _asmovement (Utilities|Casting|CastToMovement _returnvalue))
    (Variables|/Game/Blueprint/Movement.Movement_C|SetDialog _asmovement "Here lies Ina Michelle ")
    (Variables|Default|Settalkint 1)
    (elif (== (Variables|Default|Gettalkint) 1)
      (bind _asmovement_2 (Utilities|Casting|CastToMovement _returnvalue))
      (Variables|/Game/Blueprint/Movement.Movement_C|SetDialog _asmovement_2 "Died of omnipotence.")
      (Variables|Default|Settalkint 2)
      (elif (== (Variables|Default|Gettalkint) 2)
        (Variables|Default|Settalkint 0)
        (CallFunction|EndDialog)))))

(fn ConstructionScript)