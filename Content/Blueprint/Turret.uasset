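; Turret actor that tracks the player character and fires projectiles while the player is within attack range.
; Each tick it smoothly turns its Top component toward the player with RInterpTo when in range, then updates the range flag by distance.
; A self-recalling shoot event starts on BeginPlay, spawning projectiles from Top with pitch offset 180 degrees at the fire rate, or rechecking every half second when out of range.
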(event Custom|TurretRotation
  (bind _returnvalue (Game|GetPlayerCharacter 0))
  (bind _top (Variables|Default|Gettop))
  (bind _returnvalue_2 (Transformation|GetWorldLocation _top))
  (bind _returnvalue_3 (Transformation|GetActorLocation _returnvalue))
  (bind _returnvalue_4 (Math|Rotator|FindLookatRotation _returnvalue_2 _returnvalue_3))
  (bind (_roll _pitch _yaw) (Math|Rotator|BreakRotator _returnvalue_4))
  ;[1 1 1] this gets the player location, looks at the player and rotats with it if the player is in shooting range
  (if (Variables|Default|GetInRange)
    (Transformation|SetWorldRotation (Variables|Default|Gettop) (Math|Interpolation|RInterpTo (Transformation|GetWorldRotation (Variables|Default|Gettop)) (Math|Rotator|MakeRotator 0.0 _pitch _yaw) (Variables|Default|GetDeltaTime) (Variables|Default|GetRotationSpeed)) false false)))

(event Custom|Range
  ;[1 1 1] it collects the distance from the turrent to the character
  (if (< (Transformation|GetDistanceTo self (Game|GetPlayerCharacter 0)) (Variables|Default|GetAttackrange))
    (Variables|Default|SetInRange true)
    (else
      (Variables|Default|SetInRange false))))

(event Custom|shootPlayer
  (bind _top (Variables|Default|Gettop))
  (bind _returnvalue (Transformation|GetWorldTransform _top))
  (bind (_location _rotation _scale) (Math|Transform|BreakTransform _returnvalue))
  (bind (_roll _pitch _yaw) (Math|Rotator|BreakRotator _rotation))
  ;[1 1 1] this will shoot at the player if the player are in range
  (if (Variables|Default|GetInRange)
    (Game|SpawnActorfromClass "/Game/Blueprint/ProjectileFire.ProjectileFire_C" (Math|Transform|MakeTransform _location (Math|Rotator|MakeRotator _roll (- _pitch 1.8e+02) _yaw) _scale) "Undefined" 0 0)
    (Utilities|FlowControl|RetriggerableDelay (Variables|Default|GetFireRate))
    (CallFunction|ShootPlayer)
    (else
      (Utilities|FlowControl|RetriggerableDelay 0.5)
      (CallFunction|ShootPlayer))))

(event EventTick
  (params (DeltaSeconds :type Float%20%28single-precision%29))
  ;[1 1 1] every tick the machine launches the turret rotation and checks the range
  (Variables|Default|SetDeltaTime DeltaSeconds)
  (CallFunction|TurretRotation)
  (CallFunction|Range))

(event EventBeginPlay
  ;[1 1 1] Launch this functions when the game starts
  (CallFunction|ShootPlayer))

(fn ConstructionScript)