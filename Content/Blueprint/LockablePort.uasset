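; LockablePort is a door actor that opens on player interaction once its key-pickup flag is set.
; Overlap shows a widget while the door is closed and hides it on leaving or once opened.
; Opening disables the cube's collision and plays a timeline that lerps the whole actor from its starting rotation to a -90 degree yaw offset, both cached at BeginPlay.
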(event Custom|Opendoor
  (if (Variables|Default|GetCheck%20key%20pickup)
    (Variables|Default|Setdoor%20is%20open true)
    (Collision|SetCollisionEnabled (Variables|Default|GetCube) "NoCollision")
    (bind _dooropener (Timeline|Timeline_0 Play)
      (:Update
        (Transformation|SetActorRotation (Math|Rotator|Lerp(Rotator) (Variables|Default|GetObject%20Rotation) (Variables|Default|GetRotator%20of%20this%20obj) _dooropener))))))

(event Collision|EventActorEndOverlap
  (params (OtherActor :type Actor%20Object%20Reference))
  (Rendering|SetVisibility (Variables|Default|GetWidget) false false))

(event EventOnPlayerInteract
  (CallFunction|Opendoor)
  (if (Variables|Default|Getdoor%20is%20open)
    (Rendering|SetVisibility (Variables|Default|GetWidget) false false)))

(event Collision|EventActorBeginOverlap
  (params (OtherActor :type Actor%20Object%20Reference))
  (if (Variables|Default|Getdoor%20is%20open)
    (Rendering|SetVisibility (Variables|Default|GetWidget) false false)
    (else
      (Rendering|SetVisibility (Variables|Default|GetWidget) true false))))

(event EventBeginPlay
  (bind _returnvalue (Transformation|GetActorRotation))
  (bind (_roll _pitch _yaw) (Math|Rotator|BreakRotator _returnvalue))
  (Variables|Default|SetObject%20Rotation _returnvalue)
  (Variables|Default|SetRotator%20of%20this%20obj (Math|Rotator|MakeRotator _roll _pitch (+ _yaw -9e+01))))

(fn ConstructionScript)