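; Key pickup actor that unlocks one specific locked door and spins continuously in the level.
; On overlap with the Movement class, it casts its KeyForThisDoor reference to Lockabledoor and sets CheckKeyPickup on that door.
; It then destroys itself and plays a 2D key sound.
; Tick adds a fixed world rotation to the scene component every frame, independent of delta time.
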(event EventTick
  (params (DeltaSeconds :type Float%20%28single-precision%29))
  (Transformation|AddWorldRotation (Variables|Default|GetScene) "0,1.500000,0.000000" false false))

(event Collision|EventActorBeginOverlap
  (params (OtherActor :type Actor%20Object%20Reference))
  ;[1 1 1] if player overlap he picks up the key to unlock a specific door
  (if (== "/Game/Blueprint/Movement.Movement_C" (Utilities|GetClass OtherActor))
    (bind _aslockabledoor (Utilities|Casting|CastToLockabledoor (Variables|Default|GetKeyForThisDoor)))
    (Variables|/Game/Blueprint/Lockabledoor.Lockabledoor_C|SetCheck%20key%20pickup _aslockabledoor true)
    (Actor|DestroyActor)
    (Audio|PlaySound2D "/Game/Sound/Foley/Keys.Keys" 1.0 1.0 0.0 0 0)))

(fn ConstructionScript)