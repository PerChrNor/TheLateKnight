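; Enemy1 is an enemy actor that hurts the player on contact and is destroyed when its health reaches zero or below.
; It only loses health when the damage causer shares the player character's class, then updates the health percentage for its widget health bar.
; On actor overlap, if its Box contains the player's capsule, it applies fixed damage to the overlapping actor, gated by a one-second cooldown.
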(event Game|Damage|EventAnyDamage
  (params (Damage :type Float%20%28single-precision%29) (DamageType :type Damage%20Type%20Object%20Reference) (InstigatedBy :type Controller%20Object%20Reference) (DamageCauser :type Actor%20Object%20Reference))
  ;[1 1 1] Taking Damage
  (bind _output_get (Variables|Default|Setdamaged%20byplayer (== (Utilities|GetClass DamageCauser) (Utilities|GetClass (Game|GetPlayerCharacter 0)))))
  (if _output_get
    (Variables|Default|SetEnemyHealth (- (Variables|Default|GetEnemyHealth) (Math|Float|Truncate Damage)))
    (CallFunction|SetHPBar)
    (Math|Integer|CompareInt (Variables|Default|GetEnemyHealth)
      (:==
        _)
      (:<
        _))
    (Actor|DestroyActor)))

(event Collision|EventActorBeginOverlap
  (params (OtherActor :type Actor%20Object%20Reference))
  ;[1 1 1] Deal Damage to Player
  (bind _output_get (Variables|Default|Setis%20player (Utilities|Array|ContainsItem (Class|PrimitiveComponent|GetOverlappingComponents (Variables|Default|GetBox)) (Actor|GetComponentbyClass (Game|GetPlayerCharacter 0) "/Script/Engine.CapsuleComponent"))))
  (if _output_get
    (if (Variables|Default|Getready%20to%20dmg)
      (Variables|Default|Setready%20to%20dmg false)
      (Game|Damage|ApplyDamage OtherActor 4e+01 0 0)
      (Utilities|FlowControl|Delay 1.0)
      (Variables|Default|Setready%20to%20dmg true))))

(event EventBeginPlay
  ;[1 1 1] Widget setup
  (bind _asenemyhealth (Utilities|Casting|CastToEnemyhealth (UserInterface|GetUserWidgetObject (Variables|Default|Gethealthbar))))
  (Variables|/Game/Blueprint/Enemyhealth.Enemyhealth_C|SetOwner _asenemyhealth self))

(fn ConstructionScript)

(fn SetHPBar
  (Variables|Default|Setpercent (Math|Float|Clamp(Float) (/ (Math|Conversions|ToFloat(Integer) (Variables|Default|GetEnemyHealth)) 1e+02))))