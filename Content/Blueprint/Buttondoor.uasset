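; Buttondoor is a door actor that swings open by 90 degrees of negative yaw when its Opendoor event is called.
; BeginPlay caches the starting rotation and the target rotation.
; A timeline then lerps the actor between them.
; A PlaySound flag gates the opening cue on timeline update and clears after the first play, with the sound placed at world origin rather than at the door.
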(event Custom|Opendoor
  ;[1 1 1] Door opener slowly
  (bind _dooropener (Timeline|Timeline_0 Play)
    (:Update
      (Transformation|SetActorRotation (Math|Rotator|Lerp(Rotator) (Variables|Default|GetObject%20rotation) (Variables|Default|GetRotator%20of%20thisObj) _dooropener))
      (if (Variables|Default|Getplay%20sound)
        (Audio|PlaySoundatLocation "/Game/Sound/Foley/DoorOpening_Cue.DoorOpening_Cue" "0, 0, 0" "0, 0, 0" 1.0 1.0 0.0 0 0 0)
        (Variables|Default|Setplay%20sound false)))))

(event EventBeginPlay
  (bind _returnvalue (Transformation|GetActorRotation))
  (bind (_roll _pitch _yaw) (Math|Rotator|BreakRotator _returnvalue))
  ;[1 1 1] rotating the right direction
  (Variables|Default|SetObject%20rotation _returnvalue)
  (Variables|Default|SetRotator%20of%20thisObj (Math|Rotator|MakeRotator _roll _pitch (+ _yaw -9e+01))))

(fn ConstructionScript)