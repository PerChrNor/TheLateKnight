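; Player character Blueprint for Chaster, handling eight-way movement, ground dash, jump, sword attack, interaction and pause toggling.
; The current skeletal mesh selects the armored or unarmored AnimInstance that receives run, dash and attack flags.
; Attacks briefly enable a hitbox to damage overlapping actors, with delays gating attack and dash.
; Incoming damage reduces health, enemy hits add knockback, and death shows a widget before reloading the level.
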(event Custom|Enable%20Movement
  (Components|Activation|Activate (Variables|Character|GetCharacterMovement) false))

(event Custom|Disable%20movement
  (Components|Activation|Deactivate (Variables|Character|GetCharacterMovement)))

(event Custom|OnHit
  (bind _mesh (Variables|Character|GetMesh))
  (bind _mesh_2 (Variables|Character|GetMesh))
  (bind _mesh_3 (Variables|Character|GetMesh))
  (bind _returnvalue (Components|SkeletalMesh|GetAnimInstance _mesh))
  (bind _returnvalue_2 (Components|SkeletalMesh|GetAnimInstance _mesh_2))
  (bind _skeletalmesh (Variables|/Script/Engine.SkinnedMeshComponent|GetSkeletalMesh _mesh_3))
  (bind _returnvalue_3 (== _skeletalmesh "/Game/models/Animations/ChasterArmor/Chaster_Armoured_Ske.Chaster_Armoured_Ske"))
  ;[1 1 1] giving damage with hitbox and animation setups
  (if (Variables|Default|GetAttackDelay)
    (if _returnvalue_3
      (bind _asbpchaster_anim (Utilities|Casting|CastToBPChasterAnim _returnvalue))
      (Variables|/Game/Blueprint/AnimationBlueprint/BPChasterAnim.BPChasterAnim_C|SetAttacking _asbpchaster_anim true)
      (else
        (bind _asbpno_armor_chaster_anim (Utilities|Casting|CastToBPNoArmorChasterAnim _returnvalue))
        (Variables|/Game/Blueprint/AnimationBlueprint/BPNoArmorChasterAnim.BPNoArmorChasterAnim_C|SetAttacking _asbpno_armor_chaster_anim true)))
    (Collision|SetCollisionEnabled (Variables|Default|GetAttackBox) "QueryOnly")
    (for _array_element (Collision|GetOverlappingActors (Variables|Default|GetAttackBox) 0 :!class /Script/Engine.PrimitiveComponent)
      (if (not (== (Utilities|GetClass _array_element) "Movement_C"))
        (Game|Damage|ApplyDamage _array_element (Variables|Default|GetDamageDealt) 0 (Game|GetPlayerCharacter 0))))
    (Variables|Default|SetAttackDelay false)
    (Collision|SetCollisionEnabled (Variables|Default|GetAttackBox) "NoCollision")
    (Utilities|FlowControl|Delay 0.25)
    (if _returnvalue_3
      (bind _asbpchaster_anim_2 (Utilities|Casting|CastToBPChasterAnim _returnvalue_2))
      (Variables|/Game/Blueprint/AnimationBlueprint/BPChasterAnim.BPChasterAnim_C|SetAttacking _asbpchaster_anim_2 false)
      (else
        (bind _asbpno_armor_chaster_anim_2 (Utilities|Casting|CastToBPNoArmorChasterAnim _returnvalue_2))
        (Variables|/Game/Blueprint/AnimationBlueprint/BPNoArmorChasterAnim.BPNoArmorChasterAnim_C|SetAttacking _asbpno_armor_chaster_anim_2 false)))
    (Variables|Default|SetAttackDelay true)))

(event Custom|ArmorRunAnim
  (bind _mesh (Variables|Character|GetMesh))
  (bind _returnvalue (Components|SkeletalMesh|GetAnimInstance _mesh))
  ;[1 1 1] Movement setup + aniations
  (if (or (!= 0.0 (Input|AxisValues|Getright)) (!= 0.0 (stale Input|AxisEvents|InputAxisforward AxisValue)))
    (bind _asbpchaster_anim (Utilities|Casting|CastToBPChasterAnim _returnvalue))
    (Variables|/Game/Blueprint/AnimationBlueprint/BPChasterAnim.BPChasterAnim_C|SetCanRun _asbpchaster_anim true)
    (else
      (bind _asbpchaster_anim_2 (Utilities|Casting|CastToBPChasterAnim _returnvalue))
      (Variables|/Game/Blueprint/AnimationBlueprint/BPChasterAnim.BPChasterAnim_C|SetCanRun _asbpchaster_anim_2 false))))

(event Custom|NoArmorRunAnim
  (bind _mesh (Variables|Character|GetMesh))
  (bind _returnvalue (Components|SkeletalMesh|GetAnimInstance _mesh))
  ;[1 1 1] Movement setup + aniations
  (if (or (!= 0.0 (Input|AxisValues|Getright)) (!= 0.0 (stale Input|AxisEvents|InputAxisforward AxisValue)))
    (bind _asbpno_armor_chaster_anim (Utilities|Casting|CastToBPNoArmorChasterAnim _returnvalue))
    (Variables|/Game/Blueprint/AnimationBlueprint/BPNoArmorChasterAnim.BPNoArmorChasterAnim_C|SetCan%20Run _asbpno_armor_chaster_anim true)
    (else
      (bind _asbpno_armor_chaster_anim_2 (Utilities|Casting|CastToBPNoArmorChasterAnim _returnvalue))
      (Variables|/Game/Blueprint/AnimationBlueprint/BPNoArmorChasterAnim.BPNoArmorChasterAnim_C|SetCan%20Run _asbpno_armor_chaster_anim_2 false))))

(event Custom|Patrick
  (bind _mesh (Variables|Character|GetMesh))
  (bind _sword_mod (Variables|Default|GetSword_Mod))
  ;[1 1 1] attaches animations meshes and socket for sword
  (Class|SkinnedMeshComponent|SetSkeletalMesh _mesh "/Game/models/Animations/ChasterFix/ChasterFix_Ske__1_.ChasterFix_Ske__1_" true)
  (Components|SkeletalMesh|SetAnimInstanceClass _mesh "/Game/Blueprint/AnimationBlueprint/BPNoArmorChasterAnim.BPNoArmorChasterAnim_C")
  (Components|StaticMesh|SetStaticMesh _sword_mod "/Game/models/Animations/ChasterFix/StickSword_Mod.StickSword_Mod")
  (Transformation|AttachComponentToComponent _sword_mod (Variables|Character|GetMesh) "Swordhand" "KeepRelative" "KeepRelative" "KeepRelative" true)
  (Variables|Default|SetDamageDealt 19.0))

(event Game|Damage|EventAnyDamage
  (params (Damage :type Float%20%28single-precision%29) (DamageType :type Damage%20Type%20Object%20Reference) (InstigatedBy :type Controller%20Object%20Reference) (DamageCauser :type Actor%20Object%20Reference))
  (bind _returnvalue (Transformation|GetActorLocation DamageCauser))
  (bind _returnvalue_2 (Transformation|GetActorLocation))
  (bind _returnvalue_3 (Utilities|GetClass DamageCauser))
  (bind _returnvalue_4 (Math|Rotator|FindLookatRotation _returnvalue _returnvalue_2))
  (bind _returnvalue_5 (Math|Rotator|GetRotationXVector _returnvalue_4))
  (bind _returnvalue_6 (* _returnvalue_5 5e+03))
  (bind (_x _y) (Math|Vector|BreakVector _returnvalue_6))
  ;[1 1 1] character taking damage setup and deathscreen + death and loading map after death. character knockback
  (Variables|Default|SetPlayerHealth (- (Variables|Default|GetPlayerHealth) (Math|Float|Truncate Damage)))
  (if (or (== (Utilities|GetClass (Variables|Default|Getbpenemy)) _returnvalue_3) (== _returnvalue_3 "/Game/Blueprint/bpEnemyCPPslime.bpEnemyCPPslime_C"))
    (Character|LaunchCharacter (Math|Vector|MakeVector _x _y 0.0) false false))
  (if (<= (Variables|Default|GetPlayerHealth) 0)
    (bind _returnvalue_7 (UserInterface|CreateWidget "/Game/Blueprint/DeathScreen.DeathScreen_C"))
    (UserInterface|Viewport|AddtoViewport _returnvalue_7 0)
    (Utilities|FlowControl|Delay 3.0)
    (bind _returnvalue_8 (Game|GetCurrentLevelName true))
    (Game|OpenLevel(byName) (Utilities|String|StringToName _returnvalue_8))
    (Actor|DestroyActor)))

(event Input|ActionEvents|InputActionDashButton
  (params (Key :type Key%20Structure))
  (bind _mesh (Variables|Character|GetMesh))
  (bind _returnvalue (Components|SkeletalMesh|GetAnimInstance _mesh))
  ;[1 1 1] Movement setup + aniations
  (:Pressed
    (if (Variables|Default|GetAllowToDash)
      (CallFunction|Fastjumper)
      (Utilities|FlowControl|Delay 0.2)
      (if (== (Variables|/Script/Engine.SkinnedMeshComponent|GetSkeletalMesh (Variables|Character|GetMesh)) "/Game/models/Animations/ChasterArmor/Chaster_Armoured_Ske.Chaster_Armoured_Ske")
        (bind _asbpchaster_anim (Utilities|Casting|CastToBPChasterAnim _returnvalue))
        (Variables|/Game/Blueprint/AnimationBlueprint/BPChasterAnim.BPChasterAnim_C|SetDashing _asbpchaster_anim false)
        (else
          (bind _asbpno_armor_chaster_anim (Utilities|Casting|CastToBPNoArmorChasterAnim _returnvalue))
          (Variables|/Game/Blueprint/AnimationBlueprint/BPNoArmorChasterAnim.BPNoArmorChasterAnim_C|SetDashing _asbpno_armor_chaster_anim false)))
      (Variables|Default|SetAllowToDash false)
      (Utilities|FlowControl|Delay 0.5)
      (Variables|Default|SetAllowToDash true))))

(event Input|ActionEvents|InputActionAction
  (params (Key :type Key%20Structure))
  (:Pressed
    ;[1 1 1] Movement setup + aniations
    (CallFunction|OnHit)))

(event Input|ActionEvents|InputActionJUMPS
  (params (Key :type Key%20Structure))
  (:Pressed
    (Character|Jump))
  (:Released
    (Character|StopJumping)))

(event Input|ActionEvents|InputActionInterract
  (params (Key :type Key%20Structure))
  (:Pressed
    (for _array_element (Collision|GetOverlappingActors 0 :!class /Script/Engine.Actor)
      (Class|CharacterInterract|OnPlayerInteract(Message) _array_element))))

(event Input|ActionEvents|InputActionPause/Esc
  (params (Key :type Key%20Structure))
  (bind _returnvalue (Game|GetPlayerController 0))
  ;[1 1 1] Pause widget
  (:Pressed
    (bind _aspausemenu (Utilities|Casting|CastToPausemenu (Variables|Default|GetPausemenu)))
    (Utilities|FlowControl|FlipFlop
      (:A
        (Variables|/Script/Engine.PlayerController|SetbShowMouseCursor _returnvalue true)
        (Default|Pause _aspausemenu))
      (:B
        (Variables|/Script/Engine.PlayerController|SetbShowMouseCursor _returnvalue false)
        (Default|Unpause _aspausemenu)))))

(event Input|AxisEvents|InputAxisforward
  (params (AxisValue :type Float%20%28single-precision%29))
  ;[1 1 1] Movement setup + aniations
  (if (== (Variables|/Script/Engine.SkinnedMeshComponent|GetSkeletalMesh (Variables|Character|GetMesh)) "/Game/models/Animations/ChasterArmor/Chaster_Armoured_Ske.Chaster_Armoured_Ske")
    (CallFunction|ArmorRunAnim)
    (else
      (CallFunction|NoArmorRunAnim)))
  (Pawn|Input|AddMovementInput (Math|Vector|MakeVector AxisValue (Input|AxisValues|Getright) 0.0) 1.0 false)
  (CallFunction|IfMove))

(fn ConstructionScript)

(fn IfMove
  (Math|Float|CompareFloat (Input|AxisValues|Getforward) 0.0
    (:>
      (Math|Float|CompareFloat (Input|AxisValues|Getright) 0.0
        (:>
          (Transformation|SetWorldRotation (Variables|Character|GetMesh) "0,-45.000000, 0" false false))
        (:==
          (Transformation|SetWorldRotation (Variables|Character|GetMesh) "0,-90.000000, 0" false false))
        (:<
          (Transformation|SetWorldRotation (Variables|Character|GetMesh) "0,-135.000000, 0" false false))))
    (:==
      (Math|Float|CompareFloat (Input|AxisValues|Getright) 0.0
        (:>
          (Transformation|SetWorldRotation (Variables|Character|GetMesh) "0, 0, 0" false false))
        (:<
          (Transformation|SetWorldRotation (Variables|Character|GetMesh) "0,-180.000000, 0" false false))))
    (:<
      (Math|Float|CompareFloat (Input|AxisValues|Getright) 0.0
        (:>
          (Transformation|SetWorldRotation (Variables|Character|GetMesh) "0,-315.000000, 0" false false))
        (:==
          (Transformation|SetWorldRotation (Variables|Character|GetMesh) "0,-270.000000, 0" false false))
        (:<
          (Transformation|SetWorldRotation (Variables|Character|GetMesh) "0,-225.000000, 0" false false))))))

(fn Fastjumper
  (bind _mesh (Variables|Character|GetMesh))
  (bind _mesh_2 (Variables|Character|GetMesh))
  (bind _returnvalue (Transformation|GetWorldRotation _mesh))
  (bind _returnvalue_2 (Components|SkeletalMesh|GetAnimInstance _mesh_2))
  (bind (_roll _pitch _yaw) (Math|Rotator|BreakRotator _returnvalue))
  (if (AI|Components|NavMovement|IsMovingonGround (Variables|Character|GetCharacterMovement))
    (if (== (Variables|/Script/Engine.SkinnedMeshComponent|GetSkeletalMesh (Variables|Character|GetMesh)) "/Game/models/Animations/ChasterArmor/Chaster_Armoured_Ske.Chaster_Armoured_Ske")
      (bind _asbpchaster_anim (Utilities|Casting|CastToBPChasterAnim _returnvalue_2))
      (Variables|/Game/Blueprint/AnimationBlueprint/BPChasterAnim.BPChasterAnim_C|SetDashing _asbpchaster_anim true)
      (else
        (bind _asbpno_armor_chaster_anim (Utilities|Casting|CastToBPNoArmorChasterAnim _returnvalue_2))
        (Variables|/Game/Blueprint/AnimationBlueprint/BPNoArmorChasterAnim.BPNoArmorChasterAnim_C|SetDashing _asbpno_armor_chaster_anim true)))
    (Character|LaunchCharacter (* (Math|Rotator|GetRotationXVector (Math|Rotator|MakeRotator _roll _pitch (+ _yaw 9e+01))) 1e+04) false false)))